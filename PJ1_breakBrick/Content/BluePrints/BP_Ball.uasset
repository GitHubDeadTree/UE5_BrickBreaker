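; Ball actor for a brick-breaker style game that launches itself, reports brick hits and handles its own loss.
; On BeginPlay it applies an X velocity-change impulse to its sphere and caches the player's BP_Paddle pawn.
; Hits on "brick"-tagged actors update the score through the paddle's ScoreUI.
; When destroyed, it checks lives in ScoreUI, then either has the ball spawner create a replacement or shows the game-fail widget.
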(event `self.ReceiveBeginPlay`
  (`PrimitiveComponent.AddImpulse` (`self.Sphere`) (1800.0 0.0 0.0) "None" true)
  (bind _asbp_paddle (cast `/Game/BluePrints/BP_Paddle` (`GameplayStatics.GetPlayerPawn` 0)))
  (set `self.BP_Paddle` _asbp_paddle))

(event `self.ReceiveHit`
  (params (MyComp :type "PrimitiveComponent Object Reference") (Other :type "Actor Object Reference") (OtherComp :type "PrimitiveComponent Object Reference") (bSelfMoved :type Boolean) (HitLocation :type "Vector Structure") (HitNormal :type "Vector Structure") (NormalImpulse :type "Vector Structure") (Hit :type "HitResult Structure (by ref)"))
  (if (`self.ActorHasTag` Other "brick")
    (`/Game/BluePrints/BP_UI_ScoreBar.UpdateScore` (`/Game/BluePrints/BP_Paddle.scoreUI` (`self.BP_Paddle`)))))

(event `self.ReceiveDestroyed`
  (if (>= (`/Game/BluePrints/BP_UI_ScoreBar.live` (`/Game/BluePrints/BP_Paddle.scoreUI` (`self.BP_Paddle`))) 0)
    (`/Game/BluePrints/BP_Ball_Spawner.CreatBall` (`self.BP_BallSpawner`))
    (else
      (bind _returnvalue (`|CreateWidget` "/Game/BluePrints/BP_UI_GameFail.BP_UI_GameFail_C"))
      (`UserWidget.AddToViewport` _returnvalue 0))))

(fn `UserConstructionScript`)