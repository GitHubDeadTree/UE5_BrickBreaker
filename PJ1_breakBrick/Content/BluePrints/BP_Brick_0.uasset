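; BP_Brick_0 is a breakable brick for a ball-and-brick game that loses one strength point per BP_Ball hit.
; ChangeColor maps BrickStrength to a red or green material, both at construction and after surviving hits.
; At zero strength it spawns an explosion and destroys itself, then checks whether any bricks remain.
; When none remain, the level name's last digit selects the game-finish widget for level 3, otherwise the level-pass widget.
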(event `self.ReceiveBeginPlay`)

(event `self.ReceiveHit`
  (params (MyComp :type "PrimitiveComponent Object Reference") (Other :type "Actor Object Reference") (OtherComp :type "PrimitiveComponent Object Reference") (bSelfMoved :type Boolean) (HitLocation :type "Vector Structure") (HitNormal :type "Vector Structure") (NormalImpulse :type "Vector Structure") (Hit :type "HitResult Structure (by ref)"))
  (cast `/Game/BluePrints/BP_Ball` Other)
  (set `self.brickStrength` (- (`self.brickStrength`) 1))
  (if (<= (`self.brickStrength`) 0)
    (`GameplayStatics.SpawnEmitterAtLocation` "/Game/StarterContent/Particles/P_Explosion.P_Explosion" (`self.K2_GetActorLocation`))
    (`self.K2_DestroyActor`)
    (bind _outactors (`GameplayStatics.GetAllActorsOfClass` "BP_Brick_0_C"))
    (if (== (`KismetArrayLibrary.Array_Length` _outactors) 0)
      (bind _returnvalue (`GameplayStatics.GetCurrentLevelName` true))
      (bind _result (`/Engine/EditorBlueprintResources/StandardMacros.DecrementInt` (`KismetStringLibrary.Len` _returnvalue))
        (:`  `
          (if (== (`KismetStringLibrary.Conv_StringToInt` (`KismetStringLibrary.GetSubstring` _returnvalue _result)) 3)
            (bind _returnvalue_2 (`|CreateWidget` "/Game/BluePrints/BP_UI_GameFinish.BP_UI_GameFinish_C"))
            (else
              (bind _returnvalue_3 (`|CreateWidget` "/Game/BluePrints/BP_UI_GamePass.BP_UI_GamePass_C"))))
          (`UserWidget.AddToViewport` _returnvalue_3 0)
          (`UserWidget.AddToViewport` _returnvalue_2 0))))
    (else
      (`self.changeColor`))))

(fn `changeColor`
  (bind _cube (`self.Cube`))
  (switch `int` (`self.brickStrength`)
    (:`1`
      (`PrimitiveComponent.SetMaterial` _cube 0 "/Game/Materials/MT_Inst_Red.MT_Inst_Red"))
    (:`2`
      (`PrimitiveComponent.SetMaterial` _cube 0 "/Game/Materials/MT_Inst_Green.MT_Inst_Green"))))

(fn `UserConstructionScript`
  (`self.changeColor`))