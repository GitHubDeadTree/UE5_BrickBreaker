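; BP_Brick_3 is a brick variant whose color reflects its BrickStrength.
; On BeginPlay it creates a dynamic instance of the green material on its Cube.
; ChangeMartrial scales BrickStrength into capped RGB channels, sets the material's color parameter and assigns it to the Cube.
; The construction script, BeginPlay and the ChangeColor override all run this update, with ChangeColor then calling its parent.
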(event `self.ReceiveBeginPlay`
  (`parent.ReceiveBeginPlay`)
  (bind _returnvalue (`PrimitiveComponent.CreateDynamicMaterialInstance` (`self.Cube`) 0 "/Game/Materials/MT_Inst_Green.MT_Inst_Green" "None"))
  (set `self.dynamicMaterial` _returnvalue)
  (`self.changeMartrial`))

(fn `changeColor`
  (`self.changeMartrial`)
  (`parent.changeColor`))

(fn `changeMartrial`
  (bind _dynamicmaterial (`self.dynamicMaterial`))
  (bind _brickstrength (`self.brickStrength`))
  (`MaterialInstanceDynamic.SetVectorParameterValue` _dynamicmaterial "color" (`KismetMathLibrary.Conv_ColorToLinearColor` (make `Color` (`KismetMathLibrary.Conv_IntToByte` (`KismetMathLibrary.Min` (* _brickstrength 9.5) 255)) (`KismetMathLibrary.Conv_IntToByte` (`KismetMathLibrary.Min` (`KismetMathLibrary.FTrunc` (* _brickstrength 10.2)) 255)) (`KismetMathLibrary.Conv_IntToByte` (`KismetMathLibrary.Min` (`KismetMathLibrary.FTrunc` (* _brickstrength 6.3)) 255)) 255)))
  (`PrimitiveComponent.SetMaterial` (`self.Cube`) 0 _dynamicmaterial))

(fn `setColor`
  (`self.changeMartrial`))

(fn `UserConstructionScript`
  (`parent.UserConstructionScript`)
  (`self.setColor`))