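; BP_Paddle is the player-controlled paddle for a brick-breaker game, which also creates the score bar UI.
; On BeginPlay it adds the IPM_BreakBrick Enhanced Input mapping context, then creates the score widget, shows it and stores it in ScoreUI.
; IP_Move slides the Cube component along local Z by input times PaddleSpeed, swept for collision and not scaled by delta time.
; The IP_Shoot event has no logic.
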(event `self.ReceiveBeginPlay`
  (bind `_as玩家控制器` (cast `PlayerController` (`self.GetController`)))
  (bind _returnvalue (pcsubsystem `EnhancedInputLocalPlayerSubsystem` `_as玩家控制器`))
  (`/Engine/EditorBlueprintResources/StandardMacros.IsValid` _returnvalue
    (:`Is Valid`
      (`EnhancedInputSubsystemInterface.AddMappingContext` _returnvalue "/Game/Input/IPM_BreakBrick.IPM_BreakBrick" 0 (struct))
      (bind _returnvalue_2 (`|CreateWidget` "/Game/BluePrints/BP_UI_ScoreBar.BP_UI_ScoreBar_C"))
      (`UserWidget.AddToViewport` _returnvalue_2 0)
      (set `self.scoreUI` _returnvalue_2))))

(event `EnhancedInput|/Game/Input/IP_Move`
  (params (ActionValue :type "Float (double-precision)") (ElapsedSeconds :type "Float (double-precision)") (TriggeredSeconds :type "Float (double-precision)") (InputAction :type "InputAction Object Reference" :default "/Game/Input/IP_Move.IP_Move"))
  (:`Triggered`
    (`SceneComponent.K2_AddLocalOffset` (`self.Cube`) (`KismetMathLibrary.MakeVector` 0.0 0.0 (* ActionValue (`self.PaddleSpeed`))) true false)))

(event `EnhancedInput|/Game/Input/IP_Shoot`
  (params (ActionValue :type Boolean) (ElapsedSeconds :type "Float (double-precision)") (TriggeredSeconds :type "Float (double-precision)") (InputAction :type "InputAction Object Reference" :default "/Game/Input/IP_Shoot.IP_Shoot")))

(fn `UserConstructionScript`)